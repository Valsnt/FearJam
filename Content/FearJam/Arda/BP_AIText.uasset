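; BP_AIText is a dialogue actor that shows lines of speech in a SpeechBubble widget, hidden on BeginPlay.
; Any overlap with its Capsule reveals the bubble and loads the DT_SPeech row named by the CurrentText index into WID_SpeechBubble.
; Pressing Enter increments the index and swaps in the next row's text, with no check for overlap.
; Nothing in the graph hides the bubble again or resets the index.
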(event OnComponentBeginOverlap(Capsule)
  (params (OverlappedComponent :type Primitive%20Component%20Object%20Reference) (OtherActor :type Actor%20Object%20Reference) (OtherComp :type Primitive%20Component%20Object%20Reference) (OtherBodyIndex :type Integer) (bFromSweep :type Boolean) (SweepResult :type Hit%20Result%20Structure%20%28by%20ref%29))
  (bind _speechbubble (Variables|Default|GetSpeechBubble))
  (bind _returnvalue (Utilities|GetDataTableRow "/Game/FearJam/Arda/DT_SPeech.DT_SPeech" (Utilities|String|StringToName (Utilities|String|ToString(Integer) (Variables|Default|GetCurrentText))))
    (:then
      (Rendering|SetVisibility _speechbubble true false)
      (bind _aswid_speech_bubble (Utilities|Casting|CastToWID_SpeechBubble (UserInterface|GetUserWidgetObject _speechbubble)))
      (Variables|/Game/FearJam/Arda/WID_SpeechBubble.WID_SpeechBubble_C|SetCharecterSpeech _aswid_speech_bubble (Utilities|Struct|BreakSTR_speech _returnvalue)))))

(event EventBeginPlay
  (Rendering|SetVisibility (Variables|Default|GetSpeechBubble) false false))

(event Collision|EventActorBeginOverlap
  (params (OtherActor :type Actor%20Object%20Reference)))

(event EventTick
  (params (DeltaSeconds :type Float%20%28single-precision%29)))

(event Input|KeyboardEvents|Enter
  (params (Key :type Key%20Structure))
  (:Pressed
    (bind _result (Math|Integer|IncrementInt (Variables|Default|GetCurrentText))
      (:%20%20
        (bind _returnvalue (Utilities|GetDataTableRow "/Game/FearJam/Arda/DT_SPeech.DT_SPeech" (Utilities|String|StringToName (Utilities|String|ToString(Integer) _result)))
          (:then
            (bind _aswid_speech_bubble (Utilities|Casting|CastToWID_SpeechBubble (UserInterface|GetUserWidgetObject (Variables|Default|GetSpeechBubble))))
            (Variables|/Game/FearJam/Arda/WID_SpeechBubble.WID_SpeechBubble_C|SetCharecterSpeech _aswid_speech_bubble (Utilities|Struct|BreakSTR_speech _returnvalue))))))))

(fn ConstructionScript)