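; Slot-based inventory actor that stores items as class and amount pairs and creates the main inventory widget on BeginPlay.
; AddItem recursively fills free stacks up to a maximum size, then empty slots, returning any leftover.
; Remove, swap and split functions edit the slot array and refresh affected slot widgets by index.
; Using an item spawns its class as an actor and fires its EventOnUse, while show/hide toggles the widget.
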(event Custom|UpdateSlotAtIndex
  (params (Index :type Integer))
  (Default|UpdateSlot (Utilities|Array|Get(acopy) (Variables|/Game/FearJam/InventorySystem/Widgets/InventoryWidget.InventoryWidget_C|GetSlotsWidgets (Variables|Default|GetInventoryWidget)) Index)))

(event Custom|UseItemAtIndex
  (params (Index :type Integer))
  (bind _slots (Variables|Default|GetSlots))
  (bind _output (Utilities|Array|Get(acopy) _slots Index))
  (bind _itemclass (Utilities|Struct|BreakS_InventorySlots _output))
  (if (Utilities|IsValidClass _itemclass)
    (bind _returnvalue (Game|SpawnActorfromClass _itemclass (Math|Transform|MakeTransform "0, 0, 0" "0, 0, 0" "1,1,1") "AlwaysSpawn" 0 self Index 0))
    (Default|EventonUse _returnvalue)))

(event EventBeginPlay
  (Utilities|Array|Resize (Variables|Default|GetSlots) (Variables|Default|GetAmountOfSlots))
  (bind _returnvalue (UserInterface|CreateWidget "/Game/FearJam/InventorySystem/Widgets/MainInventoryWidget.MainInventoryWidget_C" 0 self (Variables|Default|GetSlotsPerRow)))
  (bind _output_get (Variables|Default|SetMainWidget _returnvalue))
  (Variables|Default|SetInventoryWidget (Variables|/Game/FearJam/InventorySystem/Widgets/MainInventoryWidget.MainInventoryWidget_C|GetInventoryWidget _output_get))
  (UserInterface|Viewport|AddtoViewport (Variables|Default|GetMainWidget) 0))

(event Collision|EventActorBeginOverlap
  (params (OtherActor :type Actor%20Object%20Reference)))

(event EventTick
  (params (DeltaSeconds :type Float%20%28single-precision%29)))

(fn ConstructionScript)

(fn IsSlotEmpty?
  (params (Index :type Integer))
  (return (not (Utilities|IsValidClass (.ItemClass (Utilities|Struct|BreakS_InventorySlots (Utilities|Array|Get(acopy) (Variables|Default|GetSlots) Index)))))))

(fn GetItemInfoatIndex
  (params (Index :type Integer))
  (bind _slots (Variables|Default|GetSlots))
  (bind _output (Utilities|Array|Get(acopy) _slots Index))
  (bind (_itemclass _amount) (Utilities|Struct|BreakS_InventorySlots _output))
  (if (Utilities|IsValidClass _itemclass)
    (return true (.ItemInfo (Utilities|GetClassDefaults _itemclass)) _amount)
    (else
      (return true (.ItemInfo (Utilities|GetClassDefaults _itemclass)) _amount))))

(fn SearchEmptySlot
  (bind (_array_element _array_index) (Utilities|Array|ForEachLoopwithBreak (Variables|Default|GetSlots) :!label _label)
    (:LoopBody
      (if (not (Utilities|IsValidClass (.ItemClass (Utilities|Struct|BreakS_InventorySlots _array_element))))
        (LocalVariables|SetLocalBool true)
        (LocalVariables|SetLocalIndex _array_index)
        (goto _label Break)))
    (:Completed
      (return (LocalVariables|GetLocalBool) (LocalVariables|GetLocalIndex)))))

(fn SearchFreeStack
  (params (ItemClass :type BP%20Master%20Item%20Class%20Reference))
  (bind (_array_element _array_index) (Utilities|Array|ForEachLoopwithBreak (Variables|Default|GetSlots) :!label _label)
    (:LoopBody
      (if (Utilities|IsValidClass (.ItemClass (Utilities|Struct|BreakS_InventorySlots _array_element)))
        (if (and (== (.ItemClass (Utilities|Struct|BreakS_InventorySlots _array_element)) ItemClass) (< (.Amount (Utilities|Struct|BreakS_InventorySlots _array_element)) (Variables|Default|GetMaxStackSize)))
          (LocalVariables|SetLocalBool true)
          (LocalVariables|SetLocalIndex _array_index)
          (goto _label Break))))
    (:Completed
      (return (LocalVariables|GetLocalBool) (LocalVariables|GetLocalIndex)))))

(fn AddItem
  (params (ItemClass :type BP%20Master%20Item%20Class%20Reference) (Amount :type Integer))
  (LocalVariables|SetLocalClass ItemClass)
  (LocalVariables|SetLocalAmount Amount)
  (if (.canBeStacked (Utilities|Struct|BreakS_ItemInfo (Utilities|Array|Get(acopy) (.ItemInfo (Utilities|GetClassDefaults ItemClass)) Amount)))
    (bind (_success _index) (CallFunction|SearchFreeStack (LocalVariables|GetLocalClass)))
    (if _success
      (LocalVariables|SetFoundIndex _index)
      (if (>= (+ (.Amount (Utilities|Struct|BreakS_InventorySlots (Utilities|Array|Get(acopy) (Variables|Default|GetSlots) (LocalVariables|GetFoundIndex)))) (LocalVariables|GetLocalAmount)) (Variables|Default|GetMaxStackSize))
        (LocalVariables|SetLocalAmount (- (+ (.Amount (Utilities|Struct|BreakS_InventorySlots (Utilities|Array|Get(acopy) (Variables|Default|GetSlots) (LocalVariables|GetFoundIndex)))) (LocalVariables|GetLocalAmount)) (Variables|Default|GetMaxStackSize)))
        (Utilities|Array|SetArrayElem (Variables|Default|GetSlots) (LocalVariables|GetFoundIndex) (Utilities|Struct|MakeS_InventorySlots (LocalVariables|GetLocalClass) (Variables|Default|GetMaxStackSize)))
        (CallFunction|UpdateSlotatIndex (LocalVariables|GetFoundIndex))
        (bind _rest (CallFunction|AddItem (LocalVariables|GetLocalClass) (LocalVariables|GetLocalAmount)))
        (return true _rest)
        (else
          (Utilities|Array|SetArrayElem (Variables|Default|GetSlots) (LocalVariables|GetFoundIndex) (Utilities|Struct|MakeS_InventorySlots (LocalVariables|GetLocalClass) (+ (.Amount (Utilities|Struct|BreakS_InventorySlots (Utilities|Array|Get(acopy) (Variables|Default|GetSlots) (LocalVariables|GetFoundIndex)))) (LocalVariables|GetLocalAmount))))
          (CallFunction|UpdateSlotatIndex (LocalVariables|GetFoundIndex))
          (return true 0)))
      (else
        (bind (_success_2 _index_2) (CallFunction|SearchEmptySlot))
        (if _success_2
          (bind _output_get (LocalVariables|SetFoundIndex _index_2))
          (if (> (LocalVariables|GetLocalAmount) (Variables|Default|GetMaxStackSize))
            (Utilities|Array|SetArrayElem (Variables|Default|GetSlots) _output_get (Utilities|Struct|MakeS_InventorySlots (LocalVariables|GetLocalClass) (Variables|Default|GetMaxStackSize)))
            (CallFunction|UpdateSlotatIndex (LocalVariables|GetFoundIndex))
            (bind _rest_2 (CallFunction|AddItem (LocalVariables|GetLocalClass) (- (Variables|Default|GetMaxStackSize) (LocalVariables|GetLocalAmount))))
            (return true _rest_2)
            (else
              (Utilities|Array|SetArrayElem (Variables|Default|GetSlots) (LocalVariables|GetFoundIndex) (Utilities|Struct|MakeS_InventorySlots (LocalVariables|GetLocalClass) (LocalVariables|GetLocalAmount)))
              (CallFunction|UpdateSlotatIndex (LocalVariables|GetFoundIndex))
              (return true 0)))
          (else
            (return false (LocalVariables|GetLocalAmount))))))
    (else
      (bind (_success_3 _index_3) (CallFunction|SearchEmptySlot))
      (if _success_3
        (bind _output_get_2 (LocalVariables|SetFoundIndex _index_3))
        (Utilities|Array|SetArrayElem (Variables|Default|GetSlots) _output_get_2 (Utilities|Struct|MakeS_InventorySlots (LocalVariables|GetLocalClass) 1))
        (CallFunction|UpdateSlotatIndex (LocalVariables|GetFoundIndex))
        (if (> (LocalVariables|GetLocalAmount) 1)
          (bind _rest_3 (CallFunction|AddItem (LocalVariables|GetLocalClass) (- (LocalVariables|GetLocalAmount) 1)))
          (return true _rest_3)
          (else
            (return true 0)))
        (else
          (return false (LocalVariables|GetLocalAmount)))))))

(fn GetAmountatIndex
  (params (Index :type Integer))
  (return (.Amount (Utilities|Struct|BreakS_InventorySlots (Utilities|Array|Get(acopy) (Variables|Default|GetSlots) Index)))))

(fn ShowInventory
  (Widget|SetVisibility (Variables|Default|GetInventoryWidget) "Visible")
  (Variables|Default|SetIsVisible true)
  (Widget|SetIsEnabled (Variables|Default|GetInventoryWidget) true)
  (return))

(fn HideInventory
  (Widget|SetVisibility (Variables|Default|GetInventoryWidget) "Hidden")
  (Variables|Default|SetIsVisible false)
  (Widget|SetIsEnabled (Variables|Default|GetInventoryWidget) false)
  (return))

(fn RemoveItematIndex
  (params (Index :type Integer) (Amount :type Integer))
  (bind _slots (Variables|Default|GetSlots))
  (LocalVariables|SetLocalIndex Index)
  (LocalVariables|SetLocalAmount Amount)
  (if (and (not (CallFunction|IsSlotEmpty? (LocalVariables|GetLocalIndex))) (> (LocalVariables|GetLocalAmount) 0))
    (bind _amount (CallFunction|GetAmountatIndex (LocalVariables|GetLocalIndex)))
    (if (>= (LocalVariables|GetLocalAmount) _amount)
      (Utilities|Array|SetArrayElem (Variables|Default|GetSlots) (LocalVariables|GetLocalIndex) (Utilities|Struct|MakeS_InventorySlots 0 0))
      (CallFunction|UpdateSlotatIndex (LocalVariables|GetLocalIndex))
      (return true)
      (else
        (Utilities|Array|SetArrayElem _slots (LocalVariables|GetLocalIndex) (Utilities|Struct|MakeS_InventorySlots (.ItemClass (Utilities|Struct|BreakS_InventorySlots (Utilities|Array|Get(acopy) _slots (LocalVariables|GetLocalIndex)))) (- (.Amount (Utilities|Struct|BreakS_InventorySlots (Utilities|Array|Get(acopy) _slots (LocalVariables|GetLocalIndex)))) (LocalVariables|GetLocalAmount))))
        (CallFunction|UpdateSlotatIndex (LocalVariables|GetLocalIndex))
        (return true)))
    (else
      (return false))))

(fn SwapSlots
  (params (Index1 :type Integer) (Index2 :type Integer))
  (bind _slots (Variables|Default|GetSlots))
  (bind _returnvalue (Utilities|Array|LastIndex _slots))
  (LocalVariables|SetLocalIndex1 Index1)
  (LocalVariables|SetLocalIndex2 Index2)
  (if (or (> (LocalVariables|GetLocalIndex1) _returnvalue) (> (LocalVariables|GetLocalIndex2) _returnvalue))
    (return false)
    (else
      (LocalVariables|SetLocalSlot2 (Utilities|Array|Get(acopy) (Variables|Default|GetSlots) (LocalVariables|GetLocalIndex2)))
      (Utilities|Array|SetArrayElem (Variables|Default|GetSlots) (LocalVariables|GetLocalIndex2) (Utilities|Array|Get(acopy) (Variables|Default|GetSlots) (LocalVariables|GetLocalIndex1)))
      (Utilities|Array|SetArrayElem (Variables|Default|GetSlots) (LocalVariables|GetLocalIndex1) (LocalVariables|GetLocalSlot2))
      (CallFunction|UpdateSlotatIndex (LocalVariables|GetLocalIndex1))
      (CallFunction|UpdateSlotatIndex (LocalVariables|GetLocalIndex2))
      (return false))))

(fn SplitStack
  (params (StackIndex :type Integer) (Amount :type Integer))
  (bind _slots (Variables|Default|GetSlots))
  (LocalVariables|SetLocalStackIndex StackIndex)
  (LocalVariables|SetLocalAmount Amount)
  (if (CallFunction|IsSlotEmpty? (LocalVariables|GetLocalStackIndex))
    (return true)
    (else
      (bind (_emptyslot_ _iteminfo _amount) (CallFunction|GetItemInfoatIndex (LocalVariables|GetLocalStackIndex)))
      (if (and (.canBeStacked (Utilities|Struct|BreakS_ItemInfo (Utilities|Array|Get(acopy) _iteminfo (LocalVariables|GetLocalStackIndex)))) (> _amount (LocalVariables|GetLocalAmount)))
        (bind (_success _index) (CallFunction|SearchEmptySlot))
        (if _success
          (LocalVariables|SetLocalFoundIndex _index)
          (Utilities|Array|SetArrayElem _slots (LocalVariables|GetLocalStackIndex) (Utilities|Struct|MakeS_InventorySlots (.itemclass (Utilities|Array|Get(acopy) _slots (LocalVariables|GetLocalStackIndex))) (- (.amount (Utilities|Array|Get(acopy) _slots (LocalVariables|GetLocalStackIndex))) (LocalVariables|GetLocalAmount))))
          (Utilities|Array|SetArrayElem (Variables|Default|GetSlots) (LocalVariables|GetLocalFoundIndex) (Utilities|Struct|MakeS_InventorySlots (.itemclass (Utilities|Array|Get(acopy) _slots (LocalVariables|GetLocalStackIndex))) (LocalVariables|GetLocalAmount)))
          (CallFunction|UpdateSlotatIndex (LocalVariables|GetLocalStackIndex))
          (CallFunction|UpdateSlotatIndex (LocalVariables|GetLocalFoundIndex))
          (return true)
          (else
            (return false)))
        (else
          (return false))))))