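; BP_MasterItem is the base item actor for the inventory system, defining what happens when an item is used.
; EventOnUse prints the name of the used item from ItemInfo, then asks the Inventory to remove one unit at the item's Index.
; The actor destroys itself only if that removal returns true.
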(event Custom|EventOnUse
  (Development|PrintString (Utilities|String|Append "You used " (Utilities|String|ToString(Text) (.name (Utilities|Array|Get(acopy) (Variables|Default|GetItemInfo) (Variables|Default|GetIndex))))))
  (bind _success (Default|RemoveItematIndex (Variables|Default|GetInventory) (Variables|Default|GetIndex) 1))
  (if _success
    (Actor|DestroyActor)))

(event EventBeginPlay)

(event Collision|EventActorBeginOverlap
  (params (OtherActor :type Actor%20Object%20Reference)))

(event EventTick
  (params (DeltaSeconds :type Float%20%28single-precision%29)))

(fn ConstructionScript)