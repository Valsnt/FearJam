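; Day/night cycle actor that fades a directional light and spawns Vampire enemies at night.
; Tick starts delayed timelines through DoOnce gates, flipping IsDay at light intensity thresholds to alternate phases.
; At night, Tick also tops Vampires up to four at a fixed location.
; As dawn brightens past the threshold, each timeline update destroys the first Vampire found.
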(event EventBeginPlay
  (Variables|Default|SetIsDay? true))

(event Collision|EventActorBeginOverlap
  (params (OtherActor :type Actor%20Object%20Reference)))

(event EventTick
  (params (DeltaSeconds :type Float%20%28single-precision%29))
  (bind _directionallight (Variables|Default|GetDirectionalLight))
  ;[1 1 1] DayNightCycle and Spawning Enemies at Night
  (bind _outactors (Actor|GetAllActorsOfClass "/Game/FearJam/Enemies/Vampires.Vampires_C"))
  (if (< (Utilities|Array|Length _outactors) 4)
    (CallFunction|SpawnEnemies))
  (if (Variables|Default|GetIsDay?)
    (Utilities|FlowControl|DoOnce false :!label _label
      (:Completed
        (Utilities|FlowControl|Delay (Variables|Default|GetDayTimer))
        (bind _daytonight (Timeline|DatToNight PlayFromStart)
          (:Update
            (bind _output_get (Variables|Default|SetDirectionalLightIntensity _daytonight))
            (Rendering|Components|Light|SetIntensity _directionallight _output_get)
            (if (== (Variables|Default|GetDirectionalLightIntensity) 0.01)
              (Variables|Default|SetIsDay? false)
              (goto _label_2 Reset))))))
    (else
      (Utilities|FlowControl|DoOnce false :!label _label_2
        (:Completed
          (Utilities|FlowControl|Delay (Variables|Default|GetNightTimer))
          (bind _daytonight_2 (Timeline|NightToDay PlayFromStart)
            (:Update
              (bind _output_get_2 (Variables|Default|SetDirectionalLightIntensity _daytonight_2))
              (Rendering|Components|Light|SetIntensity _directionallight _output_get_2)
              (if (>= (Variables|Default|GetDirectionalLightIntensity) 0.5)
                (Variables|Default|SetIsDay? true)
                (bind _outactors_2 (Actor|GetAllActorsOfClass "/Game/FearJam/Enemies/Vampires.Vampires_C"))
                (Actor|DestroyActor (Utilities|Array|Get(acopy) _outactors_2))
                (goto _label Reset)))))))))

(fn ConstructionScript)

(fn SpawnEnemies
  (if (not (Variables|Default|GetIsDay?))
    (bind _outactors (Actor|GetAllActorsOfClass "/Game/FearJam/Enemies/Vampires.Vampires_C"))
    (if (< (Utilities|Array|Length _outactors) 4)
      (AI|SpawnAIFromClass "/Game/FearJam/Enemies/Vampires.Vampires_C" 0 "1000.000000,200.000000, 0" "0, 0, 0" false))))