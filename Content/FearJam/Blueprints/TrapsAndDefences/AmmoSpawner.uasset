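; Ammo spawner actor that places an Ammo pickup at its root location and respawns it after it is gone.
; BeginPlay spawns the first pickup immediately with the configured AmmoAmount.
; Tick calls DoesPickUpExist and, when none is found, waits RespawnTime before spawning again.
; The check uses GetAllActorsOfClass, so any Ammo actor in the level blocks respawning, not only this spawner's own.
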(event Collision|EventActorBeginOverlap
  (params (OtherActor :type Actor%20Object%20Reference)))

(event EventTick
  (params (DeltaSeconds :type Float%20%28single-precision%29))
  ;[1 1 1] Spawn Collectible
  (bind _itemexists (CallFunction|DoesPickUpExist))
  (if (not _itemexists)
    (Utilities|FlowControl|Delay (Variables|Default|GetRespawnTime))
    (Game|SpawnActorfromClass "/Game/FearJam/Blueprints/TrapsAndDefences/Ammo.Ammo_C" (Math|Conversions|ToTransform(Vector) (Transformation|GetWorldLocation (Variables|Default|GetDefaultSceneRoot))) "Undefined" 0 (Variables|Default|GetAmmoAmount) 0)))

(event EventBeginPlay
  ;[1 1 1] Spawn Collectible
  (Game|SpawnActorfromClass "/Game/FearJam/Blueprints/TrapsAndDefences/Ammo.Ammo_C" (Math|Conversions|ToTransform(Vector) (Transformation|GetWorldLocation (Variables|Default|GetDefaultSceneRoot))) "Undefined" 0 (Variables|Default|GetAmmoAmount) 0))

(fn ConstructionScript)

(fn DoesPickUpExist
  (bind _outactors (Actor|GetAllActorsOfClass "/Game/FearJam/Blueprints/TrapsAndDefences/Ammo.Ammo_C"))
  (if (> (Utilities|Array|Length _outactors) 0)
    (Variables|Default|SetItemExists true)
    (else
      (Variables|Default|SetItemExists false)))
  (return (Variables|Default|GetItemExists)))