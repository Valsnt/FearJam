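; PlantSpawner is a spawner actor that keeps a collectible PickUpItem available, spawning one at its root location on BeginPlay.
; Each Tick calls DoesPickUpExist and, when none is found, waits RespawnTime before spawning another with the configured ItemToAdd and Amount.
; The existence check uses GetAllActorsOfClass across the world, so any PickUpItem anywhere, not just this spawner's own, blocks respawning.
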(event Collision|EventActorBeginOverlap
  (params (OtherActor :type Actor%20Object%20Reference)))

(event EventTick
  (params (DeltaSeconds :type Float%20%28single-precision%29))
  ;[1 1 1] Spawn Collectible
  (bind _itemexists (CallFunction|DoesPickUpExist))
  (if (not _itemexists)
    (Utilities|FlowControl|Delay (Variables|Default|GetRespawnTime))
    (Game|SpawnActorfromClass (Variables|Default|GetPickUpItem) (Math|Conversions|ToTransform(Vector) (Transformation|GetWorldLocation (Variables|Default|GetDefaultSceneRoot))) "Undefined" 0 (Variables|Default|GetItemToAdd) (Variables|Default|GetAmount) 0)))

(event EventBeginPlay
  ;[1 1 1] Spawn Collectible
  (Game|SpawnActorfromClass (Variables|Default|GetPickUpItem) (Math|Conversions|ToTransform(Vector) (Transformation|GetWorldLocation (Variables|Default|GetDefaultSceneRoot))) "Undefined" 0 (Variables|Default|GetItemToAdd) (Variables|Default|GetAmount) 0))

(fn ConstructionScript)

(fn DoesPickUpExist
  (bind _outactors (Actor|GetAllActorsOfClass (Variables|Default|GetPickUpItem)))
  (if (> (Utilities|Array|Length _outactors) 0)
    (Variables|Default|SetItemExists true)
    (else
      (Variables|Default|SetItemExists false)))
  (return (Variables|Default|GetItemExists)))