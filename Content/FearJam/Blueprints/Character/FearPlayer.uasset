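; FearPlayer is the player character, handling movement, an inventory and plant placement (commented as garlic).
; On BeginPlay it spawns an Inventory actor linked back to itself, which the I key shows and hides.
; Movement axes follow control yaw.
; Left click scans the slots for items matching the referenced plant class, uses each match and spawns that plant at the cursor's visibility-trace hit, using the pawn's rotation.
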(event EventBeginPlay
  ;[1 1 1] Create Inv Ref
  (bind _returnvalue (Game|SpawnActorfromClass "/Game/FearJam/InventorySystem/Blueprints/Inventory.Inventory_C" (Math|Transform|MakeTransform "0, 0, 0" "0, 0, 0" "1,1,1") "AlwaysSpawn" 0 16 self 4 0))
  (Variables|Default|SetInventoryReference _returnvalue))

(event Collision|EventActorBeginOverlap
  (params (OtherActor :type Actor%20Object%20Reference))
  ;[1 1 1] Create Inv Ref
)

(event Input|AxisEvents|InputAxisMoveForward
  (params (AxisValue :type Float%20%28single-precision%29))
  ;[1 1 1] Movement
  (Pawn|Input|AddMovementInput (Math|Vector|GetForwardVector (Math|Rotator|MakeRotator 0.0 0.0 (.Yaw (Math|Rotator|BreakRotator (Pawn|GetControlRotation :!class /Script/Engine.Pawn))))) AxisValue false))

(event Input|AxisEvents|InputAxisMoveRight
  (params (AxisValue :type Float%20%28single-precision%29))
  ;[1 1 1] Movement
  (Pawn|Input|AddMovementInput (Math|Vector|GetRightVector (Math|Rotator|MakeRotator 0.0 0.0 (.Yaw (Math|Rotator|BreakRotator (Pawn|GetControlRotation :!class /Script/Engine.Pawn))))) AxisValue false))

(event Input|MouseEvents|LeftMouseButton
  (params (Key :type Key%20Structure))
  (bind _plantrefence (Variables|Default|GetPlantRefence))
  ;[1 1 1] Spawn Garlic and Remove one from Inventory
  (:Pressed
    (for (_array_element _array_index) (Variables|/Game/FearJam/InventorySystem/Blueprints/Inventory.Inventory_C|GetSlots (Variables|Default|GetInventoryReference))
      (if (Utilities|IsValidClass (.itemclass _array_element))
        (for _array_element_2 (.ItemInfo (Utilities|GetClassDefaults (.itemclass _array_element)))
          (if (Utilities|Enum|Equal(Enum) (Utilities|GetClassDefaults _plantrefence) (.name _array_element_2))
            (Default|UseItematIndex (Variables|Default|GetInventoryReference) _array_index)
            (Game|SpawnActorfromClass _plantrefence (Math|Transform|MakeTransform (.Location (Collision|BreakHitResult (.HitResult (Game|Player|GetHitResultUnderCursorbyChannel (Game|GetPlayerController 0) "TraceTypeQuery1" true)))) (Transformation|GetActorRotation (Game|Player|GetPlayerPawn 0))) "Undefined" 0 0)))))))

(event Input|KeyboardEvents|I
  (params (Key :type Key%20Structure))
  (bind _inventoryreference (Variables|Default|GetInventoryReference))
  ;[1 1 1] bring up inv
  (:Pressed
    (if (Variables|/Game/FearJam/InventorySystem/Blueprints/Inventory.Inventory_C|GetIsVisible (Variables|Default|GetInventoryReference))
      (Default|HideInventory _inventoryreference)
      (else
        (Default|ShowInventory _inventoryreference)))))

(fn ConstructionScript)