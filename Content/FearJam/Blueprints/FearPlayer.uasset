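; FearPlayer is the player pawn Blueprint for FearJam, handling movement and inventory access.
; On BeginPlay it spawns an Inventory actor, passes itself as that actor's player reference and stores the result.
; Forward and right axis inputs move the pawn relative to the control rotation's yaw only.
; The I key shows or hides the inventory based on its IsVisible state.
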(event EventBeginPlay
  ;[1 1 1] Create Inv Ref
  (bind _returnvalue (Game|SpawnActorfromClass "/Game/FearJam/InventorySystem/Blueprints/Inventory.Inventory_C" (Math|Transform|MakeTransform "0, 0, 0" "0, 0, 0" "1,1,1") "AlwaysSpawn" 0 20 self 4 0))
  (Variables|Default|SetInventoryReference _returnvalue))

(event Collision|EventActorBeginOverlap
  (params (OtherActor :type Actor%20Object%20Reference))
  ;[1 1 1] Create Inv Ref
)

(event Input|AxisEvents|InputAxisMoveForward
  (params (AxisValue :type Float%20%28single-precision%29))
  ;[1 1 1] Movement
  (Pawn|Input|AddMovementInput (Math|Vector|GetForwardVector (Math|Rotator|MakeRotator 0.0 0.0 (.Yaw (Math|Rotator|BreakRotator (Pawn|GetControlRotation :!class /Script/Engine.Pawn))))) AxisValue false))

(event Input|AxisEvents|InputAxisMoveRight
  (params (AxisValue :type Float%20%28single-precision%29))
  ;[1 1 1] Movement
  (Pawn|Input|AddMovementInput (Math|Vector|GetRightVector (Math|Rotator|MakeRotator 0.0 0.0 (.Yaw (Math|Rotator|BreakRotator (Pawn|GetControlRotation :!class /Script/Engine.Pawn))))) AxisValue false))

(event Input|KeyboardEvents|I
  (params (Key :type Key%20Structure))
  (bind _inventoryreference (Variables|Default|GetInventoryReference))
  ;[1 1 1] bring up inv
  (:Pressed
    (if (Variables|/Game/FearJam/InventorySystem/Blueprints/Inventory.Inventory_C|GetIsVisible (Variables|Default|GetInventoryReference))
      (Default|HideInventory _inventoryreference)
      (else
        (Default|ShowInventory _inventoryreference)))))

(fn ConstructionScript)