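; Light switch Blueprint that turns a group of lights on or off together.
; ToggleLights checks the LightsOn flag, then loops over the Lights array, setting each light component's intensity to zero or a fixed bright value and flipping the flag inside the loop.
; The event graph and construction script are empty, so nothing in this Blueprint calls the toggle.
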(event EventBeginPlay)

(event Collision|EventActorBeginOverlap
  (params (OtherActor :type Actor%20Object%20Reference)))

(event EventTick
  (params (DeltaSeconds :type Float%20%28single-precision%29)))

(fn ConstructionScript)

(fn ToggleLights
  (if (Variables|Default|GetbLightsOn)
    (for _array_element (Variables|Default|GetLights)
      (Rendering|Components|Light|SetIntensity (Variables|/Script/Engine.Light|GetLightComponent _array_element) 0.0)
      (Variables|Default|SetbLightsOn false))
    (else
      (for _array_element_2 (Variables|Default|GetLights)
        (Rendering|Components|Light|SetIntensity (Variables|/Script/Engine.Light|GetLightComponent _array_element_2) 5e+04)
        (Variables|Default|SetbLightsOn true)))))